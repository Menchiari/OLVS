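; BP_EnemyLady is a two-phase Tempest combat enemy that fights with hand weapons and a gun.
; On BeginPlay it swaps in LadyCombatComponent, adds defense and poise modifiers, builds both hand traces and registers a phase 2 condition.
; Events switch to phase 2 swords with denser trace sockets, toggle trails and particles, crossfade weapon opacity and fire projectiles at the target's pelvis.
; It also provides a screen-space lock-on widget.
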(event Custom|Toggle%20Opacity%20Materials
  (params (NewParam :type Boolean))
  (if NewParam
    (bind _newtrack_0 (Timeline|Timeline_0 Play)
      (:Update
        (Rendering|Material|SetScalarParameterValueonMaterials (Variables|Character|GetMesh) "Opacity" (Math|Float|Lerp 1.0 0.0 _newtrack_0))))
    (else
      (Timeline|Timeline_0 Reverse))))

(event Custom|Start%20Phase%202%20Equipment
  (bind _array (Utilities|Array|MakeArray "Socket" "Socket0" "Socket1" "Socket2" "Socket3" "Socket4" "Socket5" "Socket6" "Socket7" "Socket8" "Socket9" "Socket10" "Socket11" "Socket12" "Socket13" "Socket10" "Socket14" "Socket15" "Socket16" "Socket17"))
  (Rendering|SetVisibility (Variables|Default|GetLong%20Sword%20Phase%202) true false)
  (Rendering|SetVisibility (Variables|Default|GetL_Gun) false false)
  (Class|TempestBaseTraceObject|SetTraceMeshInfo (Class|TempestCollisionManagerComponent|GetTraceOfGameplayTag (Variables|Default|GetBP_TempestCollisionManager) "(TagName=\"Trace.Right Hand Weapon\")") (Variables|Default|GetR_WP) _array)
  (Class|TempestBaseTraceObject|SetTraceMeshInfo (Class|TempestCollisionManagerComponent|GetTraceOfGameplayTag (Variables|Default|GetBP_TempestCollisionManager) "(TagName=\"Trace.Left Hand Weapon\")") (Variables|Default|GetLong%20Sword%20Phase%202) _array))

(event Custom|Toggle%20Swords%20Join
  (params (Toggle :type Boolean))
  (Transformation|AttachComponentToComponent (Variables|Default|GetLong%20Sword%20Phase%202) (Variables|Character|GetMesh) (select Toggle "Smash_JointSword" "LHand_Long_Sword") "SnapToTarget" "SnapToTarget" "SnapToTarget" true))

(event Custom|Toggle%20Show%20Gun
  (params (Toggle :type Boolean))
  (if Toggle
    (bind _newtrack_0 (Timeline|Timeline_1 Play)
      (:Update
        (Rendering|Material|SetScalarParameterValueonMaterials (Variables|Default|GetL_WP_2) "Opacity" (Math|Float|Lerp 1.0 0.0 _newtrack_0))
        (Rendering|Material|SetScalarParameterValueonMaterials (Variables|Default|GetL_Gun) "Opacity" (Math|Float|Lerp 0.0 1.0 _newtrack_0))))
    (else
      (Timeline|Timeline_1 Reverse))))

(event Custom|Shoot%20Gun%20Bullet
  (bind _l_gun (Variables|Default|GetL_Gun))
  (bind _returnvalue (Transformation|GetSocketLocation _l_gun "Socket"))
  (bind _ascharacter (Utilities|Casting|CastToCharacter (Default|GetCombatTarget (Variables|Default|GetBP_TempestEnemyCombatComponent))))
  (Game|SpawnActorfromClass "/Game/TempestCombatFramework/Projectiles/BP_GunShotProjectile.BP_GunShotProjectile_C" (Math|Transform|MakeTransform _returnvalue (Math|Rotator|FindLookatRotation _returnvalue (Transformation|GetSocketLocation (Variables|/Script/Engine.Character|GetMesh _ascharacter) "pelvis")) "2.000000,2.000000,2.000000") "Undefined" self 0)
  (bind _returnvalue_2 (Effects|SpawnEmitteratLocation "/Game/Effects/ParticleSystems/Weapons/AssaultRifle/Muzzle/P_AssaultRifle_MF.P_AssaultRifle_MF" _returnvalue (Math|Rotator|FindLookatRotation _returnvalue (Transformation|GetSocketLocation (Variables|/Script/Engine.Character|GetMesh _ascharacter) "pelvis")) "4.000000,4.000000,4.000000"))
  (Utilities|FlowControl|Delay 0.05)
  (Components|DestroyComponent _returnvalue_2))

(event Custom|Toggle%20Phase%202%20Trail
  (params (Togle%20Value :type Boolean) (Hand%20 :type Gameplay%20Tag%20Structure))
  (if Togle%20Value
    (|SwitchGameplayTag Hand%20
      (:Trace.Right%20Hand%20Weapon
        (bind _returnvalue (Effects|SpawnEmitterAttached "/Game/TrailMaster/Particle/Trail/Trail_011-020/Trail_018/P_Trail_018.P_Trail_018" (Variables|Default|GetR_WP) "Trail_Start"))
        (Effects|Particles|Trails|BeginTrails _returnvalue "Trail_Start" "Trail_end" "ETrailWidthMode_FromCentre" 1.0)
        (bind _returnvalue_2 (Effects|SpawnEmitterAttached "/Game/TrailMaster/Particle/Trail/Trail_011-020/Trail_018/P_Trail_018.P_Trail_018" (Variables|Default|GetR_WP) "Trail_end"))
        (Effects|Particles|Trails|BeginTrails _returnvalue_2 "Trail_end" "Trail_end2" "ETrailWidthMode_FromCentre" 1.0))
      (:Trace.Left%20Hand%20Weapon
        (bind _returnvalue_3 (Effects|SpawnEmitterAttached "/Game/TrailMaster/Particle/Trail/Trail_011-020/Trail_018/P_Trail_018.P_Trail_018" (Variables|Default|GetLong%20Sword%20Phase%202) "Trail_Start"))
        (Effects|Particles|Trails|BeginTrails _returnvalue_3 "Trail_Start" "Trail_end" "ETrailWidthMode_FromCentre" 1.0)
        (bind _returnvalue_4 (Effects|SpawnEmitterAttached "/Game/TrailMaster/Particle/Trail/Trail_011-020/Trail_018/P_Trail_018.P_Trail_018" (Variables|Default|GetLong%20Sword%20Phase%202) "Trail_end"))
        (Effects|Particles|Trails|BeginTrails _returnvalue_4 "Trail_end" "Trail_end2" "ETrailWidthMode_FromCentre" 1.0)))
    (else
      (|SwitchGameplayTag Hand%20
        (:Trace.Right%20Hand%20Weapon
          (Utilities|IsValid _returnvalue
            (:Is%20Valid
              (Effects|Particles|Trails|EndTrails _returnvalue)
              (Components|DestroyComponent _returnvalue)
              (Utilities|IsValid _returnvalue_2
                (:Is%20Valid
                  (Effects|Particles|Trails|EndTrails _returnvalue_2)
                  (Components|DestroyComponent _returnvalue_2))))))
        (:Trace.Left%20Hand%20Weapon
          (Utilities|IsValid _returnvalue_3
            (:Is%20Valid
              (Effects|Particles|Trails|EndTrails _returnvalue_3)
              (Components|DestroyComponent _returnvalue_3)
              (Utilities|IsValid _returnvalue_4
                (:Is%20Valid
                  (Effects|Particles|Trails|EndTrails _returnvalue_4)
                  (Components|DestroyComponent _returnvalue_4))))))))))

(event Custom|Toggle%20Phase%202%20Particle
  (params (Hand :type Gameplay%20Tag%20Structure) (Toggle :type Boolean))
  (bind _bp_tempestenemycombatcomponent (Variables|Default|GetBP_TempestEnemyCombatComponent))
  (bind _returnvalue (Class|TempestCombatComponent|GetCombatConditionOfGameplayTag _bp_tempestenemycombatcomponent "(TagName=\"Condition.Combat.Phase\")"))
  (Utilities|IsValid _returnvalue
    (:Is%20Valid
      (bind _returnvalue_2 (Class|TempestBaseConditionObject|GetConditionResult _returnvalue))
      (if _returnvalue_2
        (Utilities|FlowControl|Sequence
          (:then_0
            (|SwitchGameplayTag Hand
              (:Trace.Right%20Hand%20Weapon
                (if Toggle
                  (bind _returnvalue_3 (Effects|SpawnEmitterAttached "/Game/TrailMaster/Particle/Trail/Trail_011-020/Trail_018/P_Particle_018.P_Particle_018" (Variables|Default|GetR_WP) "Trail_Start"))
                  (else
                    (Utilities|IsValid _returnvalue_3
                      (:Is%20Valid
                        (Components|DestroyComponent _returnvalue_3))))))
              (:Trace.Left%20Hand%20Weapon
                (if Toggle
                  (bind _returnvalue_4 (Effects|SpawnEmitterAttached "/Game/TrailMaster/Particle/Trail/Trail_011-020/Trail_018/P_Particle_018.P_Particle_018" (Variables|Default|GetLong%20Sword%20Phase%202) "Trail_Start"))
                  (else
                    (Utilities|IsValid _returnvalue_4
                      (:Is%20Valid
                        (Components|DestroyComponent _returnvalue_4))))))))
          (:then_1
            (|SwitchGameplayTag Hand
              (:Trace.Right%20Hand%20Weapon
                (if Toggle
                  (bind _returnvalue_5 (Effects|SpawnEmitterAttached "/Game/TrailMaster/Particle/Trail/Trail_011-020/Trail_018/P_Particle_018.P_Particle_018" (Variables|Default|GetR_WP) "Trail_end"))
                  (else
                    (Utilities|IsValid _returnvalue_5
                      (:Is%20Valid
                        (Components|DestroyComponent _returnvalue_5))))))
              (:Trace.Left%20Hand%20Weapon
                (if Toggle
                  (bind _returnvalue_6 (Effects|SpawnEmitterAttached "/Game/TrailMaster/Particle/Trail/Trail_011-020/Trail_018/P_Particle_018.P_Particle_018" (Variables|Default|GetLong%20Sword%20Phase%202) "Trail_end"))
                  (else
                    (Utilities|IsValid _returnvalue_6
                      (:Is%20Valid
                        (Components|DestroyComponent _returnvalue_6))))))))
          (:then_2
            (|SwitchGameplayTag Hand
              (:Trace.Right%20Hand%20Weapon
                (if Toggle
                  (bind _returnvalue_7 (Effects|SpawnEmitterAttached "/Game/TrailMaster/Particle/Trail/Trail_011-020/Trail_018/P_Particle_018.P_Particle_018" (Variables|Default|GetR_WP) "Trail_end2"))
                  (else
                    (Utilities|IsValid _returnvalue_7
                      (:Is%20Valid
                        (Components|DestroyComponent _returnvalue_7))))))
              (:Trace.Left%20Hand%20Weapon
                (if Toggle
                  (bind _returnvalue_8 (Effects|SpawnEmitterAttached "/Game/TrailMaster/Particle/Trail/Trail_011-020/Trail_018/P_Particle_018.P_Particle_018" (Variables|Default|GetLong%20Sword%20Phase%202) "Trail_end2"))
                  (else
                    (Utilities|IsValid _returnvalue_8
                      (:Is%20Valid
                        (Components|DestroyComponent _returnvalue_8)))))))))))))

(event EventBeginPlay
  (bind _returnvalue (Actor|GetComponentbyClass "/Script/TempestCombatFramework.TempestCombatComponent"))
  (bind _array (Utilities|Array|MakeArray "Socket" "Socket0" "Socket1" "Socket2" "Socket3"))
  (|CallParentFunction)
  (Utilities|FlowControl|Delay 0.3)
  (Components|DestroyComponent (Variables|Default|GetBP_TempestEnemyCombatComponent))
  (bind _returnvalue_2 (Game|AddComponentbyClass "/Game/TempestCombatFramework/AI/Components/LadyCombatComponent.LadyCombatComponent_C" 0))
  (bind _output_get (Variables|Default|SetBP_TempestEnemyCombatComponent _returnvalue_2))
  (Default|InitAICombatComponent _output_get)
  (Rendering|Material|SetScalarParameterValueonMaterials (Variables|Default|GetL_Gun) "Opacity" 0.0)
  (bind _constructedproperty (Class|TempestCombatComponent|ConstructDefensePropertyOfClass _returnvalue "/Game/TempestCombatFramework/Actors/BP_LM_DefenseProperty.BP_LM_DefenseProperty_C"))
  (Class|TempestCombatComponent|SetDefenseProperty _returnvalue _constructedproperty)
  (Class|TempestAttributesComponents|ConstructAttributeModifierOfClass (Variables|Default|GetBP_TempestAttributesComponents) "/TempestCombatFramework/Attributes/Modifiers/BP_EnemyPoiseAttributeModifer.BP_EnemyPoiseAttributeModifer_C" (Utilities|Struct|MakeAttributeModifierProperties "(TagName=\"Attribute.Poise\")" true 2e+04 2.0))
  (bind _returnvalue_3 (Game|SpawnActorfromClass "/TempestCombatFramework/Actors/Weapons/BP_BaseWeapon.BP_BaseWeapon_C" (Math|Transform|MakeTransform "0, 0, 0" "0, 0, 0" "1.000000,1.000000,1.000000") "Undefined" self 0))
  (Default|SetEquippedWeapon (Variables|Default|GetBP_TempestEnemyCombatComponent) _returnvalue_3)
  (Utilities|FlowControl|Sequence
    (:then_0
      (bind _createdtraceobject (Class|TempestCollisionManagerComponent|ConstructTraceOfClass (Variables|Default|GetBP_TempestCollisionManager) "/TempestCombatFramework/Trace/BP_BaseTraceObject.BP_BaseTraceObject_C"))
      (Variables|/Script/TempestCombatFramework.TempestBaseTraceObject|SetTraceGameplayTag _createdtraceobject "(TagName=\"Trace.Right Hand Weapon\")")
      (Class|TempestBaseTraceObject|SetTraceMeshInfo _createdtraceobject (Variables|Default|GetR_WP) _array))
    (:then_2
      (bind _createdtraceobject_2 (Class|TempestCollisionManagerComponent|ConstructTraceOfClass (Variables|Default|GetBP_TempestCollisionManager) "/TempestCombatFramework/Trace/BP_BaseTraceObject.BP_BaseTraceObject_C"))
      (Variables|/Script/TempestCombatFramework.TempestBaseTraceObject|SetTraceGameplayTag _createdtraceobject_2 "(TagName=\"Trace.Left Hand Weapon\")")
      (Class|TempestBaseTraceObject|SetTraceMeshInfo _createdtraceobject_2 (Variables|Default|GetL_WP_2) _array))
    (:then_3
      (bind _returnvalue_4 (Game|ConstructObjectfromClass self "/Game/TempestCombatFramework/Conditions/BP_Phase2Condition.BP_Phase2Condition_C"))
      (Class|TempestCombatComponent|AddtoCombatConditions (Variables|Default|GetBP_TempestEnemyCombatComponent) _returnvalue_4))))

(event EventToggleTargetingPoint
  (params (Toggle :type Boolean))
  (if Toggle
    (Utilities|IsValid (Variables|Default|GetCreated%20Widget%20Component)
      (:Is%20Not%20Valid
        (bind _returnvalue (AddComponent|AddWidgetComponent false))
        (bind _output_get (Variables|Default|SetCreated%20Widget%20Component _returnvalue))
        (Class|WidgetComponent|SetWidgetSpace _output_get "Screen")
        (Class|WidgetComponent|SetDrawSize (Variables|Default|GetCreated%20Widget%20Component) "(X=30.000000,Y=30.000000)")
        (bind _returnvalue_2 (UserInterface|CreateWidget "/Game/TempestCombatFramework/AI/WB_LockOnPoint.WB_LockOnPoint_C"))
        (UserInterface|SetWidget (Variables|Default|GetCreated%20Widget%20Component) _returnvalue_2)
        (Transformation|AttachComponentToComponent (Variables|Default|GetCreated%20Widget%20Component) (Variables|Character|GetMesh) "pelvis" "SnapToTarget" "SnapToTarget" "SnapToTarget" true)))
    (else
      (Utilities|IsValid (Variables|Default|GetCreated%20Widget%20Component)
        (:Is%20Valid
          (Components|DestroyComponent (Variables|Default|GetCreated%20Widget%20Component)))))))

(fn ConstructionScript)

(fn GetLockonLocation
  (bind _created_widget_component (Variables|Default|GetCreated%20Widget%20Component))
  (Utilities|IsValid _created_widget_component
    (:Is%20Valid
      (return (Transformation|GetWorldLocation _created_widget_component)))
    (:Is%20Not%20Valid
      (return (+ (Transformation|GetWorldLocation (Variables|Character|GetMesh)) "0,0,105.000000")))))