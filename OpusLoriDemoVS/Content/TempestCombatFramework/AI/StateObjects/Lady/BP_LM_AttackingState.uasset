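; Attacking state for the Lady enemy AI in the Tempest Combat Framework.
; It requires a valid combat target and a runnable ability from the current phase's list, with phase 2 using its own set.
; On start, queued states take priority over performing the selected ability.
; A random roll picks the next state, weighted toward repositioning, with fallbacks through restarting the attack, closing distance and following the target.
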(event EventStartState
  (bind _tempest_state_manager_component (CallFunction|GetTempestStateManagerComponent))
  (bind _returnvalue (Class|TempestBaseStateManagerComponent|TryPerformStatesOfClass _tempest_state_manager_component (Variables|/Script/TempestCombatFramework.TempestBaseStateManagerComponent|GetQueuedStates _tempest_state_manager_component) true))
  (if (not _returnvalue)
    (Class|TempestBaseAbilityManagerComponent|PerformAbilityOfClass (Variables|/TempestCombatFramework/Characters/TCF_MasterEnemy_BP.TCF_MasterEnemy_BP_C|GetBP_TempestAbilitySystemComponent (Variables|/TempestCombatFramework/Controllers/TCF_MasterEnemy_AIC_BP.TCF_MasterEnemy_AIC_BP_C|GetMaster%20Enemy (Variables|Default|GetMaster%20Enemy%20AIC))) (CallFunction|GetSelectedAbility))))

(fn CanPerformState
  (bind _master_enemy_aic (Variables|Default|GetMaster%20Enemy%20AIC))
  (bind _master_enemy (Variables|/TempestCombatFramework/Controllers/TCF_MasterEnemy_AIC_BP.TCF_MasterEnemy_AIC_BP_C|GetMaster%20Enemy _master_enemy_aic))
  (bind _bp_tempestenemycombatcomponent (Variables|/TempestCombatFramework/Characters/TCF_MasterEnemy_BP.TCF_MasterEnemy_BP_C|GetBP_TempestEnemyCombatComponent _master_enemy))
  (Utilities|IsValid (Default|GetCombatTarget _bp_tempestenemycombatcomponent)
    (:Is%20Valid
      (switch int (Default|GetEnemyCurrentPhase _bp_tempestenemycombatcomponent)
        (:Default
          _)
        (:1
          _)
        (:2
          (bind _return_value (CallFunction|CheckAbilitiestoRun (Variables|AttackBehavior|Get2nd%20Phase%20Attack%20Abilities)))
          (return _return_value)))
      (bind _return_value_2 (CallFunction|CheckAbilitiestoRun (Variables|AttackBehavior|Get1st%20Phase%20Attack%20Abilities)))
      (return _return_value_2))
    (:Is%20Not%20Valid
      (return false))))

(fn DecideNextState
  (bind _tempest_state_manager_component (CallFunction|GetTempestStateManagerComponent))
  (bind _tempest_state_manager_component_2 (CallFunction|GetTempestStateManagerComponent))
  (|CallParentFunction)
  (switch int (Math|Random|RandomIntegerinRange 0 5)
    (:Default
      (bind _returnvalue (Class|TempestBaseStateManagerComponent|TryPerformStateOfClass (CallFunction|GetTempestStateManagerComponent) "/Game/TempestCombatFramework/AI/StateObjects/Lady/BP_LMRepositionState.BP_LMRepositionState_C" true))
      (if (not _returnvalue)
        (bind _returnvalue_2 (Class|TempestBaseStateObject|RestartState true))
        (if (not _returnvalue_2)
          (bind _returnvalue_3 (Class|TempestBaseStateManagerComponent|TryPerformStateOfClass _tempest_state_manager_component_2 "/Game/TempestCombatFramework/AI/StateObjects/Lady/BP_LM_DistanceClosureState.BP_LM_DistanceClosureState_C" true :!label _label))
          (if (not _returnvalue_3)
            (Class|TempestBaseStateManagerComponent|TryPerformStateOfClass _tempest_state_manager_component_2 (Utilities|GetClass (Class|TempestBaseStateManagerComponent|GetStateOfGameplayTag _tempest_state_manager_component_2 "(TagName=\"State.FollowTarget\")")) true)))))
    (:0
      (Class|TempestBaseStateManagerComponent|TryPerformStateOfClass _tempest_state_manager_component (Utilities|GetClass (Class|TempestBaseStateManagerComponent|GetStateOfGameplayTag _tempest_state_manager_component "(TagName=\"State.FollowTarget\")")) true))
    (:1
      (goto _label))))