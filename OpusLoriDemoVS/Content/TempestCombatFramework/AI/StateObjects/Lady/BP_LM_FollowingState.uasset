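; Following state for the Lady (LM) enemy AI in the Tempest Combat Framework.
; On start it runs a timer and tries queued states; preparation updates the AI move set.
; Each tick reapplies one follow walk speed, regardless of distance, and decides the next state once within the stop-follow distance.
; A random roll favors distance closure or attack, with closure as attack's fallback and a restart if closure fails or, on one roll, the gap remains.
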(event EventTickState
  (params (TickTime :type Float%20%28single-precision%29))
  (CallFunction|ProcessCalculations))

(event EventStartState
  (bind _tempest_state_manager_component (CallFunction|GetTempestStateManagerComponent))
  (Class|TempestBaseStateObject|StartStateTimer)
  (Class|TempestBaseStateManagerComponent|TryPerformStatesOfClass _tempest_state_manager_component (Class|TempestBaseStateManagerComponent|GetQueuedStates _tempest_state_manager_component) true))

(event EventPrepareStateValues
  (CallFunction|AdjustMovementSpeedBasedonDistance)
  (Default|CallOnUpdatedAIMoveSet (Variables|/TempestCombatFramework/Controllers/TCF_MasterEnemy_AIC_BP.TCF_MasterEnemy_AIC_BP_C|GetMaster%20Enemy (Variables|Default|GetMaster%20Enemy%20AIC)) "NewEnumerator1"))

(fn AdjustMovementSpeedBasedonDistance
  (CallFunction|CalculateDistanceDifference)
  (Variables|/Script/Engine.CharacterMovementComponent|SetMaxWalkSpeed (Variables|/Script/Engine.Character|GetCharacterMovement (Variables|/TempestCombatFramework/Controllers/TCF_MasterEnemy_AIC_BP.TCF_MasterEnemy_AIC_BP_C|GetMaster%20Enemy (Variables|Default|GetMaster%20Enemy%20AIC))) (.FollowSpeedUnderFollowThreshold (Utilities|Struct|BreakS_AIFollowBehavior (Variables|FollowingBehavior|GetFollowing%20Behavior%20Properties)))))

(fn ProcessCalculations
  (|CallParentFunction)
  (CallFunction|AdjustMovementSpeedBasedonDistance)
  (bind _returnvalue (CallFunction|CalculateDistanceDifference))
  (if (<= _returnvalue (.StopFollowAt (Utilities|Struct|BreakS_AIFollowBehavior (Variables|FollowingBehavior|GetFollowing%20Behavior%20Properties))))
    (CallFunction|DecideNextState)))

(fn DecideNextState
  (bind _tempest_state_manager_component (CallFunction|GetTempestStateManagerComponent))
  (|CallParentFunction)
  (switch int (Math|Random|RandomIntegerinRange 0 5)
    (:Default
      (bind _returnvalue (Class|TempestBaseStateManagerComponent|TryPerformStateOfClass (CallFunction|GetTempestStateManagerComponent) "/Game/TempestCombatFramework/AI/StateObjects/Lady/BP_LM_DistanceClosureState.BP_LM_DistanceClosureState_C" true :!label _label))
      (if (not _returnvalue)
        (Class|TempestBaseStateObject|RestartState false)))
    (:0
      (bind _returnvalue_2 (CallFunction|CalculateDistanceDifference))
      (if (> _returnvalue_2 (.StopFollowAt (Utilities|Struct|BreakS_AIFollowBehavior (Variables|FollowingBehavior|GetFollowing%20Behavior%20Properties))))
        (Class|TempestBaseStateObject|RestartState true)
        (else
          (goto _label))))
    (:1
      (bind _returnvalue_3 (Class|TempestBaseStateManagerComponent|TryPerformStateOfClass _tempest_state_manager_component (Utilities|GetClass (Class|TempestBaseStateManagerComponent|GetStateOfGameplayTag _tempest_state_manager_component "(TagName=\"State.Attack\")")) true :!label _label_2))
      (if (not _returnvalue_3)
        (goto _label)))
    (:2
      (goto _label_2))))