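; Sword and gun weapon pickup that equips when the player overlaps its sphere, replacing the currently equipped weapon.
; Equipping switches the anim class and moveset, registers two socketed meshes, builds sword and pelvis traces, and adds a stamina modifier.
; AttachWeaponAtIndex moves meshes between hand and back sockets; the gun slot starts without a mesh, receiving SM_Gun when the sword is stowed.
; Unequipping destroys both meshes.
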(event OnComponentBeginOverlap(Sphere)
  (params (OverlappedComponent :type Primitive%20Component%20Object%20Reference) (OtherActor :type Actor%20Object%20Reference) (OtherComp :type Primitive%20Component%20Object%20Reference) (OtherBodyIndex :type Integer) (bFromSweep :type Boolean) (SweepResult :type Hit%20Result%20Structure%20%28by%20ref%29))
  (if (== OtherActor (Game|GetPlayerCharacter 0))
    (Actor|SetOwner OtherActor)
    (CallFunction|EquipWeapon)))

(event EventEquipWeapon
  (bind _returnvalue (Components|GetOwner))
  (bind _sphere (Variables|Default|GetSphere))
  (bind _returnvalue_2 (Actor|GetComponentbyClass _returnvalue "/TempestCombatFramework/Components/BP_TempestPlayerCombatComponent.BP_TempestPlayerCombatComponent_C"))
  (bind _equipped_weapon (Default|GetEquippedWeapon _returnvalue_2))
  (Utilities|IsValid _returnvalue
    (:Is%20Valid
      (Utilities|IsValid _equipped_weapon
        (:Is%20Valid
          (CallFunction|UnEquipWeapon _equipped_weapon))
        (:Is%20Not%20Valid
          _))
      (bind _ascharacter (Utilities|Casting|CastToCharacter (Components|GetOwner)))
      (Transformation|SetRelativeLocation (Variables|/Script/Engine.Character|GetMesh _ascharacter) (- (Variables|/Script/Engine.SceneComponent|GetRelativeLocation (Variables|/Script/Engine.Character|GetMesh _ascharacter)) "0,0,3.000000") false true)
      (Class|SkeletalMeshComponent|SetAnimClass (Variables|/Script/Engine.Character|GetMesh _ascharacter) "/Game/TempestCombatFramework/CustomAnimations/Player_SwordShield_ABP.Player_SwordShield_ABP_C")
      (Class|BPIGeneralInterface|AssignMoveset(Message) (Components|SkeletalMesh|GetAnimInstance (Variables|/Script/Engine.Character|GetMesh _ascharacter)) "NewEnumerator0")
      (Utilities|FlowControl|Sequence
        (:then_0
          (bind _createdtraceobject (Class|TempestCollisionManagerComponent|ConstructTraceOfClass (Actor|GetComponentbyClass _ascharacter "/Script/TempestCombatFramework.TempestCollisionManagerComponent") "/TempestCombatFramework/Trace/BP_BaseTraceObject.BP_BaseTraceObject_C"))
          (Variables|/Script/TempestCombatFramework.TempestBaseTraceObject|SetTraceGameplayTag _createdtraceobject "(TagName=\"Trace.Right Hand Weapon\")")
          (bind _returnvalue_3 (AddComponent|AddStaticMeshComponent false))
          (Variables|Default|SetCreated%20Mesh%20Component _returnvalue_3)
          (Collision|SetCollisionEnabled (Variables|Default|GetCreated%20Mesh%20Component) "NoCollision")
          (Transformation|AttachComponentToComponent (Variables|Default|GetCreated%20Mesh%20Component) (Variables|/Script/Engine.Character|GetMesh _ascharacter) "WeaponBackSocket" "SnapToTarget" "SnapToTarget" "SnapToTarget" true)
          (Components|StaticMesh|SetStaticMesh (Variables|Default|GetCreated%20Mesh%20Component) (Variables|Default|GetSword%20Mesh))
          (Class|TempestBaseTraceObject|SetTraceMeshInfo _createdtraceobject (Variables|Default|GetCreated%20Mesh%20Component) (Utilities|Array|MakeArray "Socket 1" "Socket 2" "Socket 3" "Socket 4" "Socket 5" "Socket 6 " "Socket 7"))
          (CallFunction|RegisterWeapon (Utilities|Struct|MakeS_WeaponDetails (Variables|Default|GetCreated%20Mesh%20Component) (Variables|Default|GetSword%20Equip%20Socket) "WeaponBackSocket")))
        (:then_1
          (bind _returnvalue_4 (AddComponent|AddStaticMeshComponent false))
          (Variables|Default|SetCreated%20Mesh%20Component%202 _returnvalue_4)
          (Collision|SetCollisionEnabled (Variables|Default|GetCreated%20Mesh%20Component%202) "NoCollision")
          (Transformation|AttachComponentToComponent (Variables|Default|GetCreated%20Mesh%20Component%202) (Variables|/Script/Engine.Character|GetMesh _ascharacter) "ShieldBackSocket" "SnapToTarget" "SnapToTarget" "SnapToTarget" true)
          (Components|StaticMesh|SetStaticMesh (Variables|Default|GetCreated%20Mesh%20Component%202) 0)
          (CallFunction|RegisterWeapon (Utilities|Struct|MakeS_WeaponDetails (Variables|Default|GetCreated%20Mesh%20Component%202) (Variables|Default|GetGun%20Equip%20Socket) "ShieldBackSocket")))
        (:then_2
          (CallFunction|SetAttributes&States)
          (Default|SetEquippedWeapon (Actor|GetComponentbyClass (Components|GetOwner) "/TempestCombatFramework/Components/BP_TempestPlayerCombatComponent.BP_TempestPlayerCombatComponent_C") self)
          (Utilities|IsValid _sphere
            (:Is%20Valid
              (Components|DestroyComponent _sphere))
            (:Is%20Not%20Valid
              _))
          (bind _createdtraceobject_2 (Class|TempestCollisionManagerComponent|ConstructTraceOfClass (Actor|GetComponentbyClass _ascharacter "/Script/TempestCombatFramework.TempestCollisionManagerComponent") "/Game/TempestCombatFramework/Traces/BP_ThrownTrace.BP_ThrownTrace_C"))
          (Variables|/Script/TempestCombatFramework.TempestBaseTraceObject|SetTraceGameplayTag _createdtraceobject_2 "(TagName=\"Trace.Aoe.Self\")")
          (Class|TempestBaseTraceObject|SetTraceMeshInfo _createdtraceobject_2 (Variables|/Script/Engine.Character|GetMesh _ascharacter) (Utilities|Array|MakeArray "pelvis"))
          (Class|TempestAttributesComponents|ConstructAttributeModifierOfClass (Actor|GetComponentbyClass (Components|GetOwner) "/Script/TempestCombatFramework.TempestAttributesComponents") "/TempestCombatFramework/Attributes/Modifiers/BP_PlayerStaminaAttributeModifer.BP_PlayerStaminaAttributeModifer_C" (Utilities|Struct|MakeAttributeModifierProperties "(TagName=\"Attribute.Stamina\")" true 2e+04 0.2 3.5)))))))

(fn ConstructionScript
  (|CallParentFunction))

(fn UnEquipWeapon
  (|CallParentFunction)
  (Components|DestroyComponent (Variables|Default|GetCreated%20Mesh%20Component)))

(fn AttachWeaponatIndex
  (params (Index :type Integer) (Equip%20Slot :type Boolean))
  (bind _weapon_properties (CallFunction|GetWeaponProperties))
  (bind _output (Utilities|Array|Get(acopy) _weapon_properties Index))
  (bind (_weaponmesh _equippingsocket _unequippingsocket) (Utilities|Struct|BreakS_WeaponDetails _output))
  (if (> (Utilities|Array|Length _weapon_properties) 0)
    (bind _ascharacter (Utilities|Casting|CastToCharacter (Components|GetOwner)))
    (Utilities|IsValid _weaponmesh
      (:Is%20Valid
        (if (== Index 0)
          (if Equip%20Slot
            (Transformation|AttachComponentToComponent _weaponmesh (Variables|/Script/Engine.Character|GetMesh _ascharacter) _equippingsocket "SnapToTarget" "SnapToTarget" "SnapToTarget" true)
            (else
              (Components|StaticMesh|SetStaticMesh (Variables|Default|GetCreated%20Mesh%20Component%202) 0)
              (Components|StaticMesh|SetStaticMesh (Variables|Default|GetCreated%20Mesh%20Component%202) "/Game/TempestCombatFramework/AI/Animations/Gun_Sword_Female/Weapon/mesh/SM_Gun.SM_Gun")
              (Transformation|AttachComponentToComponent _weaponmesh (Variables|/Script/Engine.Character|GetMesh _ascharacter) _unequippingsocket "SnapToTarget" "SnapToTarget" "SnapToTarget" true)))
          (else
            (Transformation|AttachComponentToComponent _weaponmesh (Variables|/Script/Engine.Character|GetMesh _ascharacter) (select Equip%20Slot _equippingsocket _unequippingsocket) "SnapToTarget" "SnapToTarget" "SnapToTarget" true)))))))