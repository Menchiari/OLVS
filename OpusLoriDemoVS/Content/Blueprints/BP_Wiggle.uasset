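; BP_Wiggle is an actor that wiggles its root around its starting position from BeginPlay.
; WiggleHorizontal starts two timelines at different slowed play rates, each mixing three curve tracks with opposite sign patterns, scaled by Global.
; Each applies the same offset to X, Y and Z, so motion is diagonal despite the name.
; Both set absolute world location from the cached start, so they overwrite rather than add to each other.
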(event Custom|WiggleHorizontal
  (bind _initiallocation (Variables|Default|GetInitialLocation))
  (bind _global (Variables|Default|GetGlobal))
  (bind _initiallocation_0 (Variables|Default|GetInitialLocation_0))
  (bind _global_2 (Variables|Default|GetGlobal))
  (Utilities|FlowControl|Sequence
    (:then_0
      (bind (_direction _horizontal _newtrack_1 _newtrack_3) (Timeline|Horizontal Play)
        (:Update
          (Components|Timeline|SetPlayRate (Variables|Default|GetHorizontal) 0.5)
          (Transformation|SetWorldLocation (Variables|Default|GetDefaultSceneRoot) (Math|Vector|MakeVector (+ (+ (* _horizontal _global_2 1.0) (* _newtrack_1 _global_2 -1.0) (* _newtrack_3 _global_2 1.0)) (.x _initiallocation)) (+ (.y _initiallocation) (+ (* _horizontal _global_2 1.0) (* _newtrack_1 _global_2 -1.0) (* _newtrack_3 _global_2 1.0))) (+ (.z _initiallocation) (+ (* _horizontal _global_2 1.0) (* _newtrack_1 _global_2 -1.0) (* _newtrack_3 _global_2 1.0)))) false false))))
    (:then_1
      (bind (_direction_2 _horizontal_2 _newtrack_1_2 _newtrack_3_2) (Timeline|Timeline Play)
        (:Update
          (Components|Timeline|SetPlayRate (Variables|Default|GetTimeline) 0.3)
          (Transformation|SetWorldLocation (Variables|Default|GetDefaultSceneRoot) (Math|Vector|MakeVector (+ (+ (* _horizontal_2 _global -1.0) (* _newtrack_1_2 _global 1.0) (* _newtrack_3_2 _global -1.0)) (.x _initiallocation_0)) (+ (.y _initiallocation_0) (+ (* _horizontal_2 _global -1.0) (* _newtrack_1_2 _global 1.0) (* _newtrack_3_2 _global -1.0))) (+ (.z _initiallocation_0) (+ (* _horizontal_2 _global -1.0) (* _newtrack_1_2 _global 1.0) (* _newtrack_3_2 _global -1.0)))) false false))))))

(event EventBeginPlay
  (bind _defaultsceneroot (Variables|Default|GetDefaultSceneRoot))
  (bind _returnvalue (Transformation|GetWorldLocation _defaultsceneroot))
  (Variables|Default|SetInitialLocation _returnvalue)
  (Variables|Default|SetInitialLocation_0 _returnvalue)
  (CallFunction|WiggleHorizontal))

(fn ConstructionScript)