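; Actor that plays 2D music for a cinematic boss moment and fades it out on request.
; BeginPlay spawns the sound at the configured volume and keeps the audio component.
; The StopMusic event lowers the volume multiplier in small steps, re-calling itself after a short delay instead of using a timeline or built-in fade, then destroys the actor once the volume drops below zero.
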(event Custom|StopMusic
  (Utilities|FlowControl|Delay 0.1)
  (Audio|Components|Audio|SetVolumeMultiplier (Variables|Default|GetAudioComponent) (- (Variables|Default|GetVolume%20Multiplier) 0.025) :!class /Script/Engine.AudioComponent)
  (bind _output_get (Variables|Default|SetVolume%20Multiplier (- (Variables|Default|GetVolume%20Multiplier) 0.025)))
  (if (< _output_get 0.0)
    (Actor|DestroyActor)
    (else
      (CallFunction|StopMusic))))

(event EventBeginPlay
  (bind _returnvalue (Audio|SpawnSound2D (Variables|Default|GetSound) (Variables|Default|GetVolume%20Multiplier) 1.0 0.0 0))
  (Variables|Default|SetAudioComponent _returnvalue))

(fn ConstructionScript)