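; One-shot trigger volume that plays an auto-started Level Sequence on any Box overlap, with movement and look input disabled and the HUD hidden.
; If a SoundToDelete is set, a self-calling FadeOut event steps its volume multiplier down on a short delay until near zero.
; The trigger destroys itself after the fade, or immediately when no valid sound is set.
; Overlaps are not filtered or guarded against retriggering during the fade.
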(event OnComponentBeginOverlap(Box)
  (params (OverlappedComponent :type Primitive%20Component%20Object%20Reference) (OtherActor :type Actor%20Object%20Reference) (OtherComp :type Primitive%20Component%20Object%20Reference) (OtherBodyIndex :type Integer) (bFromSweep :type Boolean) (SweepResult :type Hit%20Result%20Structure%20%28by%20ref%29))
  (Sequencer|Player|CreateLevelSequencePlayer (Variables|Default|GetLevel%20Sequence) (Utilities|Struct|MakeMovieSceneSequencePlaybackSettings true "(Value=0)" 1.0 0.0 false false true true false true false false))
  (Utilities|IsValid (Variables|Default|GetSoundToDelete)
    (:Is%20Valid
      (CallFunction|FadeOut))
    (:Is%20Not%20Valid
      (Actor|DestroyActor))))

(event Custom|FadeOut
  (bind _soundtodelete (Variables|Default|GetSoundToDelete))
  (bind _audiocomponent (Variables|/Script/Engine.AmbientSound|GetAudioComponent _soundtodelete))
  (bind _volumemultiplier (Variables|/Script/Engine.AudioComponent|GetVolumeMultiplier _audiocomponent))
  (bind _returnvalue (- _volumemultiplier 0.05))
  (Audio|Components|Audio|SetVolumeMultiplier _audiocomponent _returnvalue :!class /Script/Engine.AudioComponent)
  (Utilities|FlowControl|Delay 0.1)
  (if (> _returnvalue 0.0)
    (CallFunction|FadeOut)
    (else
      (Actor|DestroyActor))))

(event EventBeginPlay)

(event Collision|EventActorBeginOverlap
  (params (OtherActor :type Actor%20Object%20Reference)))

(event EventTick
  (params (DeltaSeconds :type Float%20%28single-precision%29)))

(fn ConstructionScript)