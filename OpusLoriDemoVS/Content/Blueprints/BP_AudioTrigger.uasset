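; BP_AudioTrigger is an overlap trigger actor that plays a configured sound when the player pawn touches it.
; On overlap, it checks the Once flag and player 0's pawn, then spawns the sound with configurable volume, pitch, start time and attenuation.
; The sound plays at a referenced actor's location if valid, otherwise at a manual location, and clearing Once prevents repeat playback.
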(event EventBeginPlay)

(event Collision|EventActorBeginOverlap
  (params (OtherActor :type Actor%20Object%20Reference))
  (bind _actorlocation (Variables|Default|GetActorLocation))
  (bind _attenuation_settings (Variables|Default|GetAttenuation%20Settings))
  (if (Variables|Default|GetOnce)
    (if (Collision|IsOverlappingActor (Game|Player|GetPlayerPawn 0) :!class /Script/Engine.Actor)
      (Utilities|IsValid _actorlocation
        (:Is%20Valid
          (Audio|SpawnSoundatLocation (Variables|Default|GetSoundToPlay) (Transformation|GetActorLocation _actorlocation) "0, 0, 0" (Variables|Default|GetVolume%20Multiplier) (Variables|Default|GetPitch%20Multiplier) (Variables|Default|GetStart%20Time) _attenuation_settings 0))
        (:Is%20Not%20Valid
          (Audio|SpawnSoundatLocation (Variables|Default|GetSoundToPlay) (Variables|Default|GetManualLocation) "0, 0, 0" (Variables|Default|GetVolume%20Multiplier) (Variables|Default|GetPitch%20Multiplier) (Variables|Default|GetStart%20Time) _attenuation_settings 0)))
      (Variables|Default|SetOnce false))))

(fn ConstructionScript)