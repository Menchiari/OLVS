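; BP_EnemyGuardCastle is a castle guard actor that constantly faces the player and reacts when its Collider is overlapped.
; Every Tick, it computes a look-at rotation to the player pawn and applies the yaw, with a mesh-orientation offset, to the skeletal mesh.
; Any overlap, without filtering, sets the great sword idle animation and plays a guard sound, then a quieter short one after a delay.
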(event OnComponentBeginOverlap(Collider)
  (params (OverlappedComponent :type Primitive%20Component%20Object%20Reference) (OtherActor :type Actor%20Object%20Reference) (OtherComp :type Primitive%20Component%20Object%20Reference) (OtherBodyIndex :type Integer) (bFromSweep :type Boolean) (SweepResult :type Hit%20Result%20Structure%20%28by%20ref%29))
  (Components|Animation|SetAnimation (Variables|Default|GetSkeletalMesh) "/Game/TempestCombatFramework/AI/Animations/GreatSword/Battle/Inplace/GreatSword_Idle.GreatSword_Idle")
  (Audio|PlaySoundatLocation "/Game/AudioImported/S_Guard.S_Guard" (Transformation|GetWorldLocation (Variables|Default|GetSkeletalMesh)) "0, 0, 0" 0.5 1.0 0.0 0 0 0 0)
  (Utilities|FlowControl|Delay 1e+01)
  (Audio|PlaySoundatLocation "/Game/AudioImported/S_Guard_short.S_Guard_short" (Transformation|GetWorldLocation (Variables|Default|GetSkeletalMesh)) "0, 0, 0" 0.3 1.0 0.0 0 0 0 0))

(event EventBeginPlay)

(event Collision|EventActorBeginOverlap
  (params (OtherActor :type Actor%20Object%20Reference)))

(event EventTick
  (params (DeltaSeconds :type Float%20%28single-precision%29))
  (bind _skeletalmesh (Variables|Default|GetSkeletalMesh))
  (Transformation|SetWorldRotation _skeletalmesh (Math|Rotator|MakeRotator 0.0 0.0 (+ (.yaw (Math|Rotator|FindLookatRotation (Transformation|GetWorldLocation _skeletalmesh) (Transformation|GetActorLocation (Game|Player|GetPlayerPawn 0)))) -9e+01)) false false))

(fn ConstructionScript)