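; BP_TriggerFinalShot is a trigger actor that plays the game's closing shot when any actor overlaps it.
; It blends player 0's view to its Camera with an ease-in, then fades to black and holds once the blend time has elapsed.
; A parallel delayed chain plays the outro music, then a monologue clip.
; The overlap has no actor filter or one-shot guard.
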(event EventBeginPlay)

(event Collision|EventActorBeginOverlap
  (params (OtherActor :type Actor%20Object%20Reference))
  (bind _blend_time (Variables|Default|GetBlend%20Time))
  (Utilities|FlowControl|Sequence
    (:then_0
      (Game|Player|SetViewTargetwithBlend (Game|GetPlayerController 0) (Variables|Default|GetCamera) _blend_time "VTBlend_EaseIn" 0.75 true)
      (Utilities|FlowControl|Delay _blend_time)
      (CameraFades|StartCameraFade :self (Game|GetPlayerCameraManager 0) :ToAlpha 1.0 :bHoldWhenFinished true))
    (:then_1
      (Utilities|FlowControl|Delay 2.5)
      (Audio|PlaySound2D "/Game/AudioImported/S_Music_Outro.S_Music_Outro" 0.5 1.0 0.0 0 0)
      (Utilities|FlowControl|Delay 3.5)
      (Audio|PlaySound2D "/Game/AudioImported/S_Monologo_05.S_Monologo_05" 0.87 0.95 0.0 0 0))))

(event EventTick
  (params (DeltaSeconds :type Float%20%28single-precision%29)))

(fn ConstructionScript)