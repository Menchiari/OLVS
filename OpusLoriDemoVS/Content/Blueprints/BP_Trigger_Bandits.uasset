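; One-shot trigger that spawns a three-bandit encounter with music and timed dialogue when an actor overlaps it.
; BeginPlay snaps spawn points P1–P3 to their valid target actors, and the first overlap while Active spawns three bandit classes there with a shared enemy data asset.
; It then clears Active, alternates delayed voice lines between the first two targets (the last has no sound assigned), and destroys itself.
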(event EventBeginPlay
  (bind _p1_target (Variables|Default|GetP1_Target))
  (bind _p2_target (Variables|Default|GetP2_Target))
  (bind _p3_target (Variables|Default|GetP3_Target))
  (bind _rootcomponent (Variables|/Script/Engine.Actor|GetRootComponent _p2_target))
  (bind _rootcomponent_2 (Variables|/Script/Engine.Actor|GetRootComponent _p3_target))
  (bind _rootcomponent_3 (Variables|/Script/Engine.Actor|GetRootComponent _p1_target))
  (bind _returnvalue (Transformation|GetWorldTransform _rootcomponent))
  (bind _returnvalue_2 (Transformation|GetWorldTransform _rootcomponent_2))
  (bind _returnvalue_3 (Transformation|GetWorldTransform _rootcomponent_3))
  (Utilities|FlowControl|Sequence
    (:then_0
      (Utilities|IsValid _p1_target
        (:Is%20Valid
          (Transformation|SetWorldTransform (Variables|Default|GetP1) (Math|Transform|MakeTransform (.location _returnvalue_3) (.rotation _returnvalue_3) "1.000000,1.000000,1.000000") false false))))
    (:then_1
      (Utilities|IsValid _p2_target
        (:Is%20Valid
          (Transformation|SetWorldTransform (Variables|Default|GetP2) (Math|Transform|MakeTransform (.location _returnvalue) (.rotation _returnvalue) "1.000000,1.000000,1.000000") false false))))
    (:then_2
      (Utilities|IsValid _p3_target
        (:Is%20Valid
          (Transformation|SetWorldTransform (Variables|Default|GetP3) (Math|Transform|MakeTransform (.location _returnvalue_2) (.rotation _returnvalue_2) "1.000000,1.000000,1.000000") false false))))))

(event Collision|EventActorBeginOverlap
  (params (OtherActor :type Actor%20Object%20Reference))
  (bind _volume_multiplier (Variables|Default|GetVolume%20Multiplier))
  (bind _p1_target (Variables|Default|GetP1_Target))
  (bind _p2_target (Variables|Default|GetP2_Target))
  (bind _rootcomponent (Variables|/Script/Engine.Actor|GetRootComponent _p2_target))
  (bind _rootcomponent_2 (Variables|/Script/Engine.Actor|GetRootComponent _p1_target))
  (bind _returnvalue (Transformation|GetWorldTransform _rootcomponent))
  (bind _returnvalue_2 (Transformation|GetWorldTransform _rootcomponent_2))
  (if (Variables|Default|GetActive)
    (Game|SpawnActorfromClass "/Game/Blueprints/BP_BanditLM_1.BP_BanditLM_1_C" (Transformation|GetWorldTransform (Variables|Default|GetP1)) "Undefined" 0 "/Game/TempestCombatFramework/AI/DataAssets/Curto_EnemyDA/DA_LadyEnemy-BanditCurtoEdit.DA_LadyEnemy-BanditCurtoEdit" 0)
    (Game|SpawnActorfromClass "/Game/Blueprints/BP_BanditLM_2.BP_BanditLM_2_C" (Transformation|GetWorldTransform (Variables|Default|GetP2)) "Undefined" 0 "/Game/TempestCombatFramework/AI/DataAssets/Curto_EnemyDA/DA_LadyEnemy-BanditCurtoEdit.DA_LadyEnemy-BanditCurtoEdit" 0)
    (Game|SpawnActorfromClass "/Game/Blueprints/BP_BanditLM_3.BP_BanditLM_3_C" (Transformation|GetWorldTransform (Variables|Default|GetP3)) "Undefined" 0 "/Game/TempestCombatFramework/AI/DataAssets/Curto_EnemyDA/DA_LadyEnemy-BanditCurtoEdit.DA_LadyEnemy-BanditCurtoEdit" 0)
    (Utilities|FlowControl|Sequence
      (:then_0
        (Variables|Default|SetActive false))
      (:then_1
        (Audio|SpawnSound2D "/Game/AudioImported/S_Music_BanditsShort.S_Music_BanditsShort" 1.0 1.0 0.0 0)
        (Audio|SpawnSoundatLocation "/Game/AudioImported/S_Bandits_P2_1.S_Bandits_P2_1" (.location _returnvalue_2) "0, 0, 0" _volume_multiplier 1.0 0.0 "/Game/AudioImported/SoundAttenuation_Dialogues.SoundAttenuation_Dialogues" 0)
        (Utilities|FlowControl|Delay 6.0)
        (Audio|SpawnSoundatLocation "/Game/AudioImported/S_Bandits_P1_2.S_Bandits_P1_2" (.location _returnvalue) "0, 0, 0" _volume_multiplier 1.0 0.0 "/Game/AudioImported/SoundAttenuation_Dialogues.SoundAttenuation_Dialogues" 0)
        (Utilities|FlowControl|Delay 4.0)
        (Audio|SpawnSoundatLocation "/Game/AudioImported/S_Bandits_P2_2.S_Bandits_P2_2" (.location _returnvalue_2) "0, 0, 0" _volume_multiplier 1.0 0.0 "/Game/AudioImported/SoundAttenuation_Dialogues.SoundAttenuation_Dialogues" 0)
        (Utilities|FlowControl|Delay 5.0)
        (Audio|SpawnSoundatLocation 0 (.location _returnvalue) "0, 0, 0" _volume_multiplier 1.0 0.0 "/Game/AudioImported/SoundAttenuation_Dialogues.SoundAttenuation_Dialogues" 0)
        (Utilities|FlowControl|Delay 1e+01)
        (Actor|DestroyActor)))))

(event EventTick
  (params (DeltaSeconds :type Float%20%28single-precision%29)))

(fn ConstructionScript)